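; Base enemy character Blueprint with health, attributes and two-way combat against the player.
; BeginPlay seeds its PlayerAttribute with fixed Strength, Wisdom, Perception and Agility base values; its health assignments only copy each variable to itself.
; DealDamage casts the player character to BP_MainChar and passes BaseDamage with itself as dealer.
; TakeDamage subtracts from CurrentHealth, destroying the actor at zero or below, otherwise calling PlayAnimMontage with no montage specified.
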(event Custom|DealDamage
  (bind _asbp_main_char (Utilities|Casting|CastToBP_MainChar (Game|GetPlayerCharacter 0)))
  (Class|NinjaWizardCharacter|TakeDamagefrom _asbp_main_char (Variables|Default|GetBaseDamage) self))

(event EventBeginPlay
  (Variables|Default|SetMaxHealth (Variables|Default|GetMax%20Health))
  (Variables|Default|SetCurrent%20Health (Variables|Default|GetCurrentHealth))
  (Class|PlayerAttributeComponent|SetAttributeBaseValue (Variables|Default|GetPlayerAttribute) "Strength" 12)
  (Class|PlayerAttributeComponent|SetAttributeBaseValue (Variables|Default|GetPlayerAttribute) "Wisdom" 15)
  (Class|PlayerAttributeComponent|SetAttributeBaseValue (Variables|Default|GetPlayerAttribute) "Perception" 17)
  (Class|PlayerAttributeComponent|SetAttributeBaseValue (Variables|Default|GetPlayerAttribute) "Agility" 14))

(event Collision|EventActorBeginOverlap
  (params (OtherActor :type Actor%20Object%20Reference)))

(event EventTick
  (params (DeltaSeconds :type Float%20%28single-precision%29)))

(fn ConstructionScript)

(fn TakeDamage
  (params (Damage :type Float%20%28double-precision%29) (Attacker :type Actor%20Object%20Reference))
  (bind _output_get (Variables|Default|SetCurrent%20Health (- (Variables|Default|GetCurrent%20Health) Damage)))
  (if (<= _output_get 0.0)
    (Actor|DestroyActor)
    (else
      (Animation|PlayAnimMontage 0 1.0 "None"))))