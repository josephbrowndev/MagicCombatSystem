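; Grapple hook actor owned by BP_MainChar, drawing a cable toward that character once the hook has hit a target.
; BeginPlay caches the owning character and, if that cast succeeds, sets a short self-destruct lifespan.
; While HasHitTarget is true, Tick writes the owner's world location into the cable's EndLocation; the flag is not set in this graph.
; OnGrappleRelease destroys the hook.
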(event Custom|OnGrappleRelease
  (Actor|DestroyActor))

(event EventBeginPlay
  (bind _asbp_main_char (Utilities|Casting|CastToBP_MainChar (Components|GetOwner)))
  (Variables|Default|SetAs%20BP%20Main%20Char _asbp_main_char)
  (Actor|SetLifeSpan 5.0))

(event Collision|EventActorBeginOverlap
  (params (OtherActor :type Actor%20Object%20Reference)))

(event EventTick
  (params (DeltaSeconds :type Float%20%28single-precision%29))
  (if (Variables|Default|GetHasHitTarget?)
    (Variables|/Script/CableComponent.CableComponent|SetEndLocation (Variables|Default|GetCable) (Transformation|GetActorLocation (Components|GetOwner)))))

(fn ConstructionScript)