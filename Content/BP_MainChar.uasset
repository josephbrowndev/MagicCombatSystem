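; Main player character Blueprint that maps Enhanced Input actions to combat, traversal, inventory and magic actions.
; Dedicated components handle block, parry, dodge, grapple with directional throws, weapon slots, weapon throw and recall, and potion healing, with aiming based on control rotation.
; Inventory and radial magic menu widgets are created on input, with the radial menu removed on release.
; Fire casting only prints the selected element; the Fireball cast is unconnected.
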(event Input|EnhancedActionEvents|EnhancedInputActionIA_Block
  (params (ActionValue :type Boolean) (ElapsedSeconds :type Float%20%28double-precision%29) (TriggeredSeconds :type Float%20%28double-precision%29) (InputAction :type Input%20Action%20Object%20Reference :default "/Game/Input/Actions/CombatMovemement/IA_Block.IA_Block"))
  (bind _combatmovementcomponent (Variables|Default|GetCombatMovementComponent))
  (:Triggered
    (Class|CombatMovementComponent|StartParry _combatmovementcomponent))
  (:Started
    (Class|CombatMovementComponent|StartBlocking _combatmovementcomponent))
  (:Canceled
    (Class|CombatMovementComponent|StopBlocking _combatmovementcomponent :!label _label))
  (:Completed
    (goto _label)))

(event Input|EnhancedActionEvents|EnhancedInputActionIA_Dodge
  (params (ActionValue :type Boolean) (ElapsedSeconds :type Float%20%28double-precision%29) (TriggeredSeconds :type Float%20%28double-precision%29) (InputAction :type Input%20Action%20Object%20Reference :default "/Game/Input/Actions/CombatMovemement/IA_Dodge.IA_Dodge"))
  (bind _returnvalue (Pawn|GetControlRotation :!class /Script/Engine.Pawn))
  (bind _returnvalue_2 (Input|EnhancedActionValues|GetIA_Move))
  (bind (_x _y) (Math|Vector2D|BreakVector2D _returnvalue_2))
  (Class|CombatMovementComponent|StartDodge (Variables|Default|GetCombatMovementComponent) (+ (* (Math|Vector|GetForwardVector _returnvalue) _y) (* (Math|Vector|GetRightVector _returnvalue) _x))))

(event Input|EnhancedActionEvents|EnhancedInputActionIA_WeaponSlot4
  (params (ActionValue :type Boolean) (ElapsedSeconds :type Float%20%28double-precision%29) (TriggeredSeconds :type Float%20%28double-precision%29) (InputAction :type Input%20Action%20Object%20Reference :default "/Game/Input/Actions/WeaponActions/IA_WeaponSlot4.IA_WeaponSlot4"))
  (Class|InventoryComponent|SwitchtoWeaponSlot (Variables|Default|GetInventoryComponent) 3))

(event Input|EnhancedActionEvents|EnhancedInputActionIA_ThrowWeapon
  (params (ActionValue :type Boolean) (ElapsedSeconds :type Float%20%28double-precision%29) (TriggeredSeconds :type Float%20%28double-precision%29) (InputAction :type Input%20Action%20Object%20Reference :default "/Game/Input/Actions/WeaponActions/IA_ThrowWeapon.IA_ThrowWeapon"))
  (Class|WeaponReturnComponent|ThrowWeapon (Variables|Default|GetWeaponReturnComponent) (Class|InventoryComponent|GetCurrentWeaponSlot (Variables|Default|GetInventoryComponent)) (Math|Vector|GetForwardVector (Pawn|GetControlRotation :!class /Script/Engine.Pawn))))

(event Input|EnhancedActionEvents|EnhancedInputActionIA_RecallWeapon
  (params (ActionValue :type Boolean) (ElapsedSeconds :type Float%20%28double-precision%29) (TriggeredSeconds :type Float%20%28double-precision%29) (InputAction :type Input%20Action%20Object%20Reference :default "/Game/Input/Actions/WeaponActions/IA_RecallWeapon.IA_RecallWeapon"))
  (Class|WeaponReturnComponent|RecallAllWeapons (Variables|Default|GetWeaponReturnComponent)))

(event Input|EnhancedActionEvents|EnhancedInputActionIA_CastFire
  (params (ActionValue :type Boolean) (ElapsedSeconds :type Float%20%28double-precision%29) (TriggeredSeconds :type Float%20%28double-precision%29) (InputAction :type Input%20Action%20Object%20Reference :default "/Game/Input/Actions/MagicActions/IA_CastFire.IA_CastFire"))
  (Development|PrintString (Utilities|String|EnumtoString (Variables|Default|GetCurrentlySelectedElement))))

(event Input|EnhancedActionEvents|EnhancedInputActionIA_OpenInventory
  (params (ActionValue :type Boolean) (ElapsedSeconds :type Float%20%28double-precision%29) (TriggeredSeconds :type Float%20%28double-precision%29) (InputAction :type Input%20Action%20Object%20Reference :default "/Game/Input/Actions/Inventory/IA_OpenInventory.IA_OpenInventory"))
  (bind _returnvalue (Game|GetPlayerController 0))
  (bind _returnvalue_2 (UserInterface|CreateWidget "/Game/Content_UI/WBP_Inventory.WBP_Inventory_C" _returnvalue))
  (UserInterface|Viewport|AddtoViewport _returnvalue_2 0)
  (Input|SetInputModeGameandUI _returnvalue _returnvalue_2 "DoNotLock" false false))

(event Input|EnhancedActionEvents|EnhancedInputActionIA_UsePotion
  (params (ActionValue :type Boolean) (ElapsedSeconds :type Float%20%28double-precision%29) (TriggeredSeconds :type Float%20%28double-precision%29) (InputAction :type Input%20Action%20Object%20Reference :default "/Game/Input/Actions/Inventory/IA_UsePotion.IA_UsePotion"))
  (Class|HealingComponent|TryUsePotion (Variables|Default|GetHealingComponent) "0"))

(event Input|EnhancedActionEvents|EnhancedInputActionIA_OpenRadialMagicMenu
  (params (ActionValue :type Boolean) (ElapsedSeconds :type Float%20%28double-precision%29) (TriggeredSeconds :type Float%20%28double-precision%29) (InputAction :type Input%20Action%20Object%20Reference :default "/Game/Input/Actions/MagicActions/IA_OpenRadialMagicMenu.IA_OpenRadialMagicMenu"))
  (bind _returnvalue (Game|GetPlayerController 0))
  (:Started
    (bind _returnvalue_2 (UserInterface|CreateWidget "/Game/Content_UI/WBP_RadialMagicMenu.WBP_RadialMagicMenu_C" (Game|GetPlayerController 0)))
    (bind _output_get (Variables|Default|SetRadialMagicMenuRef _returnvalue_2))
    (UserInterface|Viewport|AddtoViewport _output_get 0))
  (:Canceled
    (bind _radialmagicmenuref (Variables|Default|GetRadialMagicMenuRef :!label _label)
      (:then
        (Widget|RemovefromParent _radialmagicmenuref)
        (Variables|/Script/Engine.PlayerController|SetbShowMouseCursor _returnvalue false)
        (Input|SetInputModeGameOnly _returnvalue false))
      (:else)))
  (:Completed
    (goto _label)))

(event Input|EnhancedActionEvents|EnhancedInputActionIA_Grapple
  (params (ActionValue :type Boolean) (ElapsedSeconds :type Float%20%28double-precision%29) (TriggeredSeconds :type Float%20%28double-precision%29) (InputAction :type Input%20Action%20Object%20Reference :default "/Game/Input/Actions/Grapple/IA_Grapple.IA_Grapple"))
  (Class|GrappleComponent|ShootGrapple (Variables|Default|GetGrappleComponent) (* (+ (Transformation|GetActorLocation) (Math|Vector|GetForwardVector (Pawn|GetControlRotation :!class /Script/Engine.Pawn))) 3e+03)))

(event Input|EnhancedActionEvents|EnhancedInputActionIA_ThrowUp
  (params (ActionValue :type Boolean) (ElapsedSeconds :type Float%20%28double-precision%29) (TriggeredSeconds :type Float%20%28double-precision%29) (InputAction :type Input%20Action%20Object%20Reference :default "/Game/Input/Actions/Grapple/IA_ThrowUp.IA_ThrowUp"))
  (Class|GrappleComponent|SetThrowDirection (Variables|Default|GetGrappleComponent) "ThrowUp"))

(event Input|EnhancedActionEvents|EnhancedInputActionIA_ThrowLeft
  (params (ActionValue :type Boolean) (ElapsedSeconds :type Float%20%28double-precision%29) (TriggeredSeconds :type Float%20%28double-precision%29) (InputAction :type Input%20Action%20Object%20Reference :default "/Game/Input/Actions/Grapple/IA_ThrowLeft.IA_ThrowLeft"))
  (Class|GrappleComponent|SetThrowDirection (Variables|Default|GetGrappleComponent) "ThrowLeft"))

(event Input|EnhancedActionEvents|EnhancedInputActionIA_ThrowRight
  (params (ActionValue :type Boolean) (ElapsedSeconds :type Float%20%28double-precision%29) (TriggeredSeconds :type Float%20%28double-precision%29) (InputAction :type Input%20Action%20Object%20Reference :default "/Game/Input/Actions/Grapple/IA_ThrowRight.IA_ThrowRight"))
  (Class|GrappleComponent|SetThrowDirection (Variables|Default|GetGrappleComponent) "ThrowRight"))

(event Input|EnhancedActionEvents|EnhancedInputActionIA_PullToPlayer
  (params (ActionValue :type Boolean) (ElapsedSeconds :type Float%20%28double-precision%29) (TriggeredSeconds :type Float%20%28double-precision%29) (InputAction :type Input%20Action%20Object%20Reference :default "/Game/Input/Actions/Grapple/IA_PullToPlayer.IA_PullToPlayer"))
  (Class|GrappleComponent|SetThrowDirection (Variables|Default|GetGrappleComponent) "PullToPlayer"))

(event Input|EnhancedActionEvents|EnhancedInputActionIA_WeaponSlot1
  (params (ActionValue :type Boolean) (ElapsedSeconds :type Float%20%28double-precision%29) (TriggeredSeconds :type Float%20%28double-precision%29) (InputAction :type Input%20Action%20Object%20Reference :default "/Game/Input/Actions/WeaponActions/IA_WeaponSlot1.IA_WeaponSlot1"))
  (Class|InventoryComponent|SwitchtoWeaponSlot (Variables|Default|GetInventoryComponent)))

(event Input|EnhancedActionEvents|EnhancedInputActionIA_WeaponSlot2
  (params (ActionValue :type Boolean) (ElapsedSeconds :type Float%20%28double-precision%29) (TriggeredSeconds :type Float%20%28double-precision%29) (InputAction :type Input%20Action%20Object%20Reference :default "/Game/Input/Actions/WeaponActions/IA_WeaponSlot2.IA_WeaponSlot2"))
  (Class|InventoryComponent|SwitchtoWeaponSlot (Variables|Default|GetInventoryComponent) 1))

(event Input|EnhancedActionEvents|EnhancedInputActionIA_WeaponSlot3
  (params (ActionValue :type Boolean) (ElapsedSeconds :type Float%20%28double-precision%29) (TriggeredSeconds :type Float%20%28double-precision%29) (InputAction :type Input%20Action%20Object%20Reference :default "/Game/Input/Actions/WeaponActions/IA_WeaponSlot3.IA_WeaponSlot3"))
  (Class|InventoryComponent|SwitchtoWeaponSlot (Variables|Default|GetInventoryComponent) 2))

(event EventBeginPlay
  (Input|AddMappingContext (PlayerController|LocalPlayerSubsystems|GetEnhancedInputLocalPlayerSubsystem (Game|GetPlayerController 0)) "/Game/Input/IMC_Default.IMC_Default" 0 "(bIgnoreAllPressedKeysUntilRelease=True,bForceImmediately=False,bNotifyUserSettings=False)"))

(event Collision|EventActorBeginOverlap
  (params (OtherActor :type Actor%20Object%20Reference)))

(event EventTick
  (params (DeltaSeconds :type Float%20%28single-precision%29)))

(fn ConstructionScript)