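; BP_MagicProjectile is a magic projectile that damages enemies on impact and expires after a three-second life span.
; Its component hit event ignores the owner character and casts other actors to BP_EnemyBase, passing damage and the owner as attacker to TakeDamage.
; An enemy hit then destroys the projectile and plays a sound at the world origin, while other hits leave it alive.
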(event OnComponentHit(ProjectilePreset)
  (params (HitComponent :type Primitive%20Component%20Object%20Reference) (OtherActor :type Actor%20Object%20Reference) (OtherComp :type Primitive%20Component%20Object%20Reference) (NormalImpulse :type Vector :default "0, 0, 0") (Hit :type Hit%20Result%20Structure%20%28by%20ref%29))
  (if (!= OtherActor (Variables|Default|GetOwnerCharacter))
    (bind _asbp_enemy_base (Utilities|Casting|CastToBP_EnemyBase OtherActor))
    (Default|TakeDamage _asbp_enemy_base (Variables|Default|GetDamage) (Variables|Default|GetOwnerCharacter))
    (Actor|DestroyActor)
    (Audio|PlaySoundatLocation 0 "0, 0, 0" "0, 0, 0" 1.0 1.0 0.0 0 0 0 0)))

(event EventBeginPlay
  (Actor|SetLifeSpan 3.0))

(event Collision|EventActorBeginOverlap
  (params (OtherActor :type Actor%20Object%20Reference)))

(event EventTick
  (params (DeltaSeconds :type Float%20%28single-precision%29)))

(fn ConstructionScript)